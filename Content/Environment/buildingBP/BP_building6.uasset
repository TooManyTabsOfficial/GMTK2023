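; Building actor that spins and swaps between its Urban and Prehistoric looks.
; SpinObject fires particles, picks a random direction and adds timeline-scaled yaw with random per-update speed, sending the flip message once as the spin starts.
; A second timeline then nudges yaw back toward zero in the same direction and re-arms the flip on finishing.
; FlipSpriteSet toggles which of the two sprite sets is hidden.
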(event `/Game/Interactable/Spinnable_BPI.SpinObject`
  (if true
    (`ActorComponent.Activate` (`self.SpinParticles`) true)
    (if (`KismetMathLibrary.RandomBool`)
      ;[1 1 1] CCW
      (bind (_direction _spinvelocityfactor) (`Timeline|Timeline_2` :!via `PlayFromStart`)
        (:`Update`
          (`self.K2_AddActorWorldRotation` (`KismetMathLibrary.MakeRotator` 0.0 0.0 (* (* (`KismetMathLibrary.Conv_IntToDouble` (`KismetMathLibrary.RandomIntegerInRange` 1 5)) -1.0) _spinvelocityfactor)))
          (`/Engine/EditorBlueprintResources/StandardMacros.DoOnce` false :!label _label
            (:`Completed`
              (message `/Game/Interactable/Spinnable_BPI.FlipSpriteSet` self))))
        (:`Finished`
          (`Timeline|Timeline_3` :!via `PlayFromStart`
            (:`Update`
              (if (not (`KismetMathLibrary.NearlyEqual_FloatFloat` (.yaw (`self.K2_GetActorRotation`)) 0.0 1.0))
                (`self.K2_AddActorWorldRotation` (struct :`Yaw` -1.0))))
            (:`Finished`
              (goto _label :!via `Reset`)))))
      (else
        ;[1 1 1] CW
        (bind (_direction_2 _spinvelocityfactor_2) (`Timeline|Timeline_0` :!via `PlayFromStart`)
          (:`Update`
            (`self.K2_AddActorWorldRotation` (`KismetMathLibrary.MakeRotator` 0.0 0.0 (* (`KismetMathLibrary.Conv_IntToDouble` (`KismetMathLibrary.RandomIntegerInRange` 1 5)) _spinvelocityfactor_2)))
            (`/Engine/EditorBlueprintResources/StandardMacros.DoOnce` false :!label _label_2
              (:`Completed`
                (message `/Game/Interactable/Spinnable_BPI.FlipSpriteSet` self))))
          (:`Finished`
            (`Timeline|Timeline_1` :!via `PlayFromStart`
              (:`Update`
                (if (not (`KismetMathLibrary.NearlyEqual_FloatFloat` (.yaw (`self.K2_GetActorRotation`)) 0.0 1.0))
                  (`self.K2_AddActorWorldRotation` (struct :`Yaw` 1.0))))
              (:`Finished`
                (goto _label_2 :!via `Reset`)))))))
    (else
      (`KismetSystemLibrary.PrintString` "Error!"))))

(event `/Game/Interactable/Spinnable_BPI.FlipSpriteSet`
  (if (`SceneComponent.bHiddenInGame` (`self.urban`))
    (`SceneComponent.SetHiddenInGame` (`self.urban`) false false)
    (`SceneComponent.SetHiddenInGame` (`self.prehistoric`) true false)
    (else
      (`SceneComponent.SetHiddenInGame` (`self.prehistoric`) false false)
      (`SceneComponent.SetHiddenInGame` (`self.urban`) true false))))

(fn `UserConstructionScript`)