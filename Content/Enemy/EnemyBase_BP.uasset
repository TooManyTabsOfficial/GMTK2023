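; EnemyBase_BP is an enemy base Blueprint that drives a sprite's idle and move flipbook animation.
; Every Tick, UpdateAnimation derives IsMoving from whether velocity is non-zero and passes it to the AnimStateMachine function.
; That function sets AnimationState to Move or Idle and selects the matching flipbook variable, which is then applied to Sprite.
; BeginPlay, overlap and the construction script contain no logic.
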(event `self.ReceiveTick`
  (params (DeltaSeconds :type "Float (single-precision)"))
  ;[1 1 1] Animation
  (`self.UpdateAnimation`))

(event `UpdateAnimation`
  ;[1 1 1] Animation
  (bind _output_get (set `self.isMoving` (> (`KismetMathLibrary.VSize` (`self.GetVelocity`)) 0.0)))
  (bind _outputflipbook (`self.Anim State Machine` _output_get))
  (`PaperFlipbookComponent.SetFlipbook` (`self.Sprite`) _outputflipbook))

(fn `Anim State Machine`
  (params (IsMoving :type Boolean))
  (returns (OutputFlipbook :type "PaperFlipbook Object Reference"))
  (if IsMoving
    (set `self.AnimationState` "NewEnumerator1")
    (else
      (set `self.AnimationState` "NewEnumerator0")))
  (return (select `/Game/Enemy/Enemy_EM` (`self.AnimationState`) :`NewEnumerator0` (`self.idleFlipbook`) :`NewEnumerator1` (`self.moveFlipbook`))))

(fn `UserConstructionScript`)