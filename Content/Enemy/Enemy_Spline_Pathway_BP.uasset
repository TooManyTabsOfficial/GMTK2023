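; Enemy pathway actor that holds a spline and returns world positions along it, likely as waypoints for enemy movement.
; GetSplineLocation increments the given index, reads that spline point's world location, stores it in SplineLocation and moves the static mesh there.
; A looping timeline with distance-along-spline interpolation remains in the graph but never runs, so movement is stepped point by point.
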(event `self.ReceiveBeginPlay`)

(event `GetSplineLocation`
  (params (SplineIndex :type Integer))
  (bind _splinelocation (`self.GetLocationOnSpline` SplineIndex))
  (set `self.SplineLocation` _splinelocation)
  (`SceneComponent.K2_SetWorldLocation` (`self.StaticMesh`) _splinelocation false false))

(fn `GetLocationOnSpline`
  (params (SplineIndex :type Integer))
  (returns (SplineLocation :type "Vector Structure"))
  (bind _result (`/Engine/EditorBlueprintResources/StandardMacros.IncrementInt` SplineIndex)
    (:`  `
      (return (`SplineComponent.GetLocationAtSplinePoint` (`self.Spline`) _result "World")))))

(fn `UserConstructionScript`)